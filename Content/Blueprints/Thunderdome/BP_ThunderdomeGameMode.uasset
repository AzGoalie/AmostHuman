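; BP_ThunderdomeGameMode is the Thunderdome game mode, which handles cleanup and respawning once the game is over.
; Tick polls the AHGameState wave state and, on GameOver, waits briefly on a Delay before destroying all BP_TrackerBot actors and restarting every player controller.
; Nothing here changes the wave state, so this sequence repeats for as long as GameOver persists.
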(event EventBeginPlay
  (|CallParentFunction) ; This node is disabled and will not be called.\nDrag off pins to build functionality.
)

(event EventTick
  (params (DeltaSeconds :type Float%20%28single-precision%29))
  (bind _asahgame_state (Utilities|Casting|CastToAHGameState (Game|GetGameState)))
  (if (Utilities|Enum|Equal(Enum) (Variables|/Script/AlmostHuman.AHGameState|GetWaveState _asahgame_state) "GameOver")
    (Utilities|FlowControl|Delay 2.0)
    ;[1 1 1] Remove all enemies
    (bind _outactors (Actor|GetAllActorsOfClass "/Game/TrackerBot/BP_TrackerBot.BP_TrackerBot_C"))
    (for _array_element _outactors
      (Actor|DestroyActor _array_element))
    ;[1 1 1] Respawn players
    (bind _outactors_2 (Actor|GetAllActorsOfClass "/Script/Engine.PlayerController"))
    (for _array_element_2 _outactors_2
      (Class|GameModeBase|RestartPlayer (Game|GetGameMode) _array_element_2))))

(fn ConstructionScript
  (|CallParentFunction))