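; BP_TestGameMode is a game mode that spawns enemy bots and awards score for kills.
; SpawnNewBot runs an EQS query for spawn locations, then spawns either a BP_AdvancedAI or, more often, a BP_TrackerBot at each returned result.
; An OnActorKilled binding made at BeginPlay gives the killer's AHPlayerState points when the victim is a non-player pawn, so player team kills earn nothing, and prints the new score.
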(event Custom|OnQueryFinishedEvent_Event_0
  (params (QueryInstance :type Env%20Query%20Instance%20Blueprint%20Wrapper%20Object%20Reference) (QueryStatus :type EEnvQueryStatus%20Enum :default "Processing"))
  (switch Utilities|FlowControl|Switch|SwitchonEEnvQueryStatus QueryStatus
    (:Success
      (for _array_element (Class|EnvQueryInstanceBlueprintWrapper|GetResultsasLocations QueryInstance)
        (Game|SpawnActorfromClass (select (<= (Math|Random|RandomFloatinRange 0.0 1e+02) 35.0) "/Game/AdvancedAI/BP_AdvancedAI.BP_AdvancedAI_C" "/Game/TrackerBot/BP_TrackerBot.BP_TrackerBot_C") (Math|Transform|MakeTransform _array_element) "AdjustIfPossibleButDontSpawnIfColliding" 0 0)))))

(event Custom|OnActorKilled_Event
  (params (VictimActor :type Actor%20Object%20Reference) (KillerActor :type Actor%20Object%20Reference) (KillerController :type Controller%20Object%20Reference))
  (Utilities|IsValid KillerController
    (:Is%20Valid
      (Utilities|IsValid KillerController
        (:Is%20Valid
          ;[1 1 1] Don't reward team killing
          (bind _aspawn (Utilities|Casting|CastToPawn VictimActor))
          (if (not (Pawn|IsPlayerControlled _aspawn))
            (bind _asahplayer_state (Utilities|Casting|CastToAHPlayerState (Variables|/Script/Engine.Pawn|GetPlayerState (Pawn|GetControlledPawn KillerController))))
            (Class|AHPlayerState|AddScore _asahplayer_state 2e+01)
            (Development|PrintString (Utilities|String|ToString(Float) (Variables|/Script/Engine.PlayerState|GetScore _asahplayer_state)) true true "(R=0.049157,G=1.000000,B=0.000000,A=1.000000)")))))))

(event EventBeginPlay
  (EventDispatchers|AssignOnActorKilled (delegate Custom|OnActorKilled_Event)))

(event EventSpawnNewBot
  (bind _returnvalue (AI|EQS|RunEQSQuery "/Game/Blueprints/EWS_FindSpawnLocation.EWS_FindSpawnLocation" self "RandomBest25Pct"))
  (EventDispatchers|AssignOnQueryFinishedEvent _returnvalue (delegate Custom|OnQueryFinishedEvent_Event_0)))

(fn ConstructionScript)